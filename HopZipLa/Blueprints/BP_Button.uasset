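; BP_Button is a pressure button that activates a linked actor when an EpicCharacter steps on it.
; Overlapping PushCollision lowers the push mesh, plays a key sound and calls SetActive(true) on ActorToEffect if valid.
; Leaving raises the mesh slightly less than it dropped, so it creeps down with each press, and never deactivates the linked actor.
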(event `self.PushCollision.OnComponentBeginOverlap`
  (params (OverlappedComponent :type "PrimitiveComponent Object Reference") (OtherActor :type "Actor Object Reference") (OtherComp :type "PrimitiveComponent Object Reference") (OtherBodyIndex :type Integer) (bFromSweep :type Boolean) (SweepResult :type "HitResult Structure (by ref)"))
  (bind _actortoeffect (`self.ActorToEffect`))
  (cast `/Game/HopZipLa/Blueprints/Charater/EpicCharacter` OtherActor)
  (`SceneComponent.K2_AddWorldOffset` (`self.StaticMeshPush`) (0.0 0.0 -10.0) false false)
  (`GameplayStatics.PlaySound2D` "/Game/Hour_of_Code/Audio/SFX_key.SFX_key" 1.0 1.0 0.0 null null)
  (`/Engine/EditorBlueprintResources/StandardMacros.IsValid` _actortoeffect
    (:`Is Valid`
      (`/Game/HopZipLa/Blueprints/Effectables/BP_Effectable.SetActive` _actortoeffect true))))

(event `self.PushCollision.OnComponentEndOverlap`
  (params (OverlappedComponent :type "PrimitiveComponent Object Reference") (OtherActor :type "Actor Object Reference") (OtherComp :type "PrimitiveComponent Object Reference") (OtherBodyIndex :type Integer))
  (cast `/Game/HopZipLa/Blueprints/Charater/EpicCharacter` OtherActor)
  (`SceneComponent.K2_AddWorldOffset` (`self.StaticMeshPush`) (0.0 0.0 9.8) false false))

(fn `UserConstructionScript`)